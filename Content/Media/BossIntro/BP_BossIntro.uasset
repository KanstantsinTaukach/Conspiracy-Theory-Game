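; BP_BossIntro plays a boss intro video sequence before the boss fight level loads.
; On BeginPlay it shows the boss intro and exit-video widgets, hides the cursor, switches to game-only input and starts the MediaSound component.
; After a fixed delay it removes the exit widget and opens the boss level whose name comes from BP_CTGGameInstance.
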(event `self.ReceiveBeginPlay`
  (bind _returnvalue (`GameplayStatics.GetPlayerController` 0))
  (bind _returnvalue_2 (`|CreateWidget` "/Game/Media/BossIntro/WBP_BossIntro.WBP_BossIntro_C"))
  (`UserWidget.AddToViewport` _returnvalue_2 0)
  (bind _returnvalue_3 (`|CreateWidget` "/Game/Media/Intro/WBP_ExitVideo.WBP_ExitVideo_C"))
  (`UserWidget.AddToViewport` _returnvalue_3 0)
  (set `PlayerController.bShowMouseCursor` false _returnvalue)
  (`WidgetBlueprintLibrary.SetInputMode_GameOnly` _returnvalue)
  (`SynthComponent.Start` (`self.MediaSound`))
  (`KismetSystemLibrary.Delay` 25.0)
  (`Widget.RemoveFromParent` _returnvalue_3)
  (bind _asbp_ctggame_instance (cast `/Game/BP_CTGGameInstance` (`GameplayStatics.GetGameInstance`)))
  (`GameplayStatics.OpenLevel` (`CTGGameInstance.GetBossLevelName` _asbp_ctggame_instance)))

(fn `UserConstructionScript`)