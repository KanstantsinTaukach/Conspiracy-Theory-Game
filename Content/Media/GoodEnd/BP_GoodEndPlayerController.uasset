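; Player controller for the good-ending video that lets the player skip to the win screen with the Space bar.
; On press, it finds and removes the WBP_GoodEnd and WBP_ExitVideo widgets and pauses the Media of the first WBP_GoodEnd instance.
; It then shows the mouse cursor, switches to UI-only input and adds a new WBP_PlayerWin widget to the viewport.
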(event `Key|SpaceBar`
  (params (Key :type "Key Structure"))
  (bind _returnvalue (`GameplayStatics.GetPlayerController` 0))
  (:`Pressed`
    (bind _foundwidgets (`WidgetBlueprintLibrary.GetAllWidgetsOfClass` "/Game/Media/GoodEnd/WBP_GoodEnd.WBP_GoodEnd_C"))
    (`Widget.RemoveFromParent` _foundwidgets)
    (`MediaPlayer.Pause` (`/Game/Media/GoodEnd/WBP_GoodEnd.Media` (`|GetArrayItem` _foundwidgets)))
    (bind _foundwidgets_2 (`WidgetBlueprintLibrary.GetAllWidgetsOfClass` "/Game/Media/Intro/WBP_ExitVideo.WBP_ExitVideo_C"))
    (`Widget.RemoveFromParent` _foundwidgets_2)
    (set `PlayerController.bShowMouseCursor` true _returnvalue)
    (`WidgetBlueprintLibrary.SetInputMode_UIOnlyEx` _returnvalue null)
    (bind _returnvalue_2 (`|CreateWidget` "/Game/UI/WBP_PlayerWin.WBP_PlayerWin_C"))
    (`UserWidget.AddToViewport` _returnvalue_2 0)))

(fn `UserConstructionScript`)