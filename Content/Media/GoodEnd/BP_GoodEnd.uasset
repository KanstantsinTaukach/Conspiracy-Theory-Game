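; BP_GoodEnd runs the good ending sequence, playing video with sound before the player win screen.
; On BeginPlay it adds the good-end and exit-video widgets, hides the cursor, switches to game-only input and starts its MediaSound.
; A fixed delay, rather than a media-finished event, times the handoff: it removes the exit-video widget, restores the cursor with UI-only input and shows WBP_PlayerWin.
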(event `self.ReceiveBeginPlay`
  (bind _returnvalue (`GameplayStatics.GetPlayerController` 0))
  (bind _returnvalue_2 (`GameplayStatics.GetPlayerController` 0))
  (bind _returnvalue_3 (`|CreateWidget` "/Game/Media/GoodEnd/WBP_GoodEnd.WBP_GoodEnd_C"))
  (`UserWidget.AddToViewport` _returnvalue_3 0)
  (bind _returnvalue_4 (`|CreateWidget` "/Game/Media/Intro/WBP_ExitVideo.WBP_ExitVideo_C"))
  (`UserWidget.AddToViewport` _returnvalue_4 0)
  (set `PlayerController.bShowMouseCursor` false _returnvalue)
  (`WidgetBlueprintLibrary.SetInputMode_GameOnly` _returnvalue)
  (`SynthComponent.Start` (`self.MediaSound`))
  (`KismetSystemLibrary.Delay` 37.0)
  (`Widget.RemoveFromParent` _returnvalue_4)
  (set `PlayerController.bShowMouseCursor` true _returnvalue_2)
  (`WidgetBlueprintLibrary.SetInputMode_UIOnlyEx` _returnvalue_2 null)
  (bind _returnvalue_5 (`|CreateWidget` "/Game/UI/WBP_PlayerWin.WBP_PlayerWin_C"))
  (`UserWidget.AddToViewport` _returnvalue_5 0))

(fn `UserConstructionScript`)