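; BP_CTGCharacter_BASE_1448 is a player character Blueprint that carries a Polaroid and can stun enemies.
; On BeginPlay it spawns BP_Polaroid with itself as owner and snaps it to the mesh's RightHandSocket.
; A hardcoded 3 key press gathers every EnemyCharacter in the world and calls Stun on each, with no range or condition check.
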(event `self.ReceiveBeginPlay`
  (bind _returnvalue (`|SpawnActorFromClass` "/Game/3DModels/polaroid/BP_Polaroid.BP_Polaroid_C" (`KismetMathLibrary.Conv_VectorToTransform` (`SceneComponent.GetSocketLocation` (`self.Mesh`) "RightHandSocket")) "AlwaysSpawn" "MultiplyWithRoot" self null))
  (`self.K2_AttachToComponent` _returnvalue (`self.Mesh`) "RightHandSocket" "SnapToTarget" "SnapToTarget" "SnapToTarget" true))

(event `Key|Three`
  (params (Key :type "Key Structure"))
  (:`Pressed`
    (bind _outactors (`GameplayStatics.GetAllActorsOfClass` "/Script/ConspiracyTheoryGame.EnemyCharacter"))
    (for _array_element _outactors
      (`EnemyCharacter.Stun` _array_element))))

(fn `UserConstructionScript`)